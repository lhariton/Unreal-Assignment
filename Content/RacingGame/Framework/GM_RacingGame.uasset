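; Game mode for a timed checkpoint racing game: the player wins on reaching the target lap count and loses when time runs out.
; BeginPlay binds to every checkpoint's events, with lap lines also advancing the lap counter that Tick polls.
; After a countdown a lose timer starts, which checkpoints re-arm with bonus time plus a HUD animation.
; Finishing disables input, silences the engine, pauses and shows a win or lose screen.
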(event `self.ReceiveTick`
  (params (DeltaSeconds :type "Float (single-precision)"))
  (if (== (`self.Lap`) 3)
    (`self.Win_CrossTheFinishLine`)))

(event `Pre-Game Start`
  (`self.Start Countdown`))

(event `self.ReceiveBeginPlay`
  (bind _outactors (`GameplayStatics.GetAllActorsOfClass` "/Game/RacingGame/Checkpoints/BP_Checkpoint.BP_Checkpoint_C"))
  (for _array_element _outactors
    (`|ExecutionSequence`
      (:`then_0`
        (add `/Game/RacingGame/Checkpoints/BP_Checkpoint.OnCheckpointCrossedWithTime` _array_element (`|CreateDelegate` :!event `CrossedCheckpoint`)))
      (:`then_1`
        (if (`/Game/RacingGame/Checkpoints/BP_Checkpoint.isLapLine` _array_element)
          (add `/Game/RacingGame/Checkpoints/BP_Checkpoint.OnCheckpointCrossedFinish` _array_element (`|CreateDelegate` :!event `New Lap`)))))))

(event `New Lap`
  (`self.AddLap` (stale `self.ReceiveBeginPlay` _array_element)))

(event `Start Countdown`
  (`KismetSystemLibrary.PrintString` "Start Countdown")
  (`KismetSystemLibrary.Delay` (`self.StartCountdownDuration`))
  (`self.Game Start`))

(event `Game Start`
  (`KismetSystemLibrary.PrintString` "Game has started")
  (`WidgetBlueprintLibrary.SetInputMode_GameOnly` (`GameplayStatics.GetPlayerController` 0))
  (bind _returnvalue (`KismetSystemLibrary.K2_SetTimerDelegate` (delegate `LoseOutOfTime`) (`self.StartTimerDuration`)))
  (set `self.TimeRemainingTimer` _returnvalue))

(event `LoseOutOfTime`
  (`self.Game Finish` false))

(event `Game Finish`
  (params (Win :type Boolean))
  (bind _returnvalue (`GameplayStatics.GetPlayerPawn` 0))
  (bind _returnvalue_2 (`GameplayStatics.GetPlayerController` 0))
  (bind _returnvalue_3 (`GameplayStatics.GetPlayerController` 0))
  (`KismetSystemLibrary.K2_ClearAndInvalidateTimerHandle` (`self.TimeRemainingTimer`))
  (`self.DisableInput` _returnvalue (`PlayerState.GetPlayerController` (`Pawn.PlayerState` _returnvalue)))
  (bind _assports_car_pawn (cast `/Game/VehicleTemplate/Blueprints/SportsCar/SportsCar_Pawn` (`GameplayStatics.GetPlayerPawn` 0)))
  (`AudioComponent.Stop` (`/Game/VehicleTemplate/Blueprints/VehicleAdvPawn.SFX_Engine` _assports_car_pawn))
  (`GameplayStatics.SetGamePaused` true)
  (if (`self.GameWon`)
    (bind _returnvalue_4 (`|CreateWidget` "/Game/RacingGame/UI/WP_WinScreen.WP_WinScreen_C"))
    (`UserWidget.AddToViewport` _returnvalue_4 0)
    (set `PlayerController.bShowMouseCursor` true _returnvalue_3)
    (`WidgetBlueprintLibrary.SetInputMode_UIOnlyEx` _returnvalue_3 (`/Game/RacingGame/UI/WP_WinScreen.Button_0` _returnvalue_4))
    (else
      (bind _returnvalue_5 (`|CreateWidget` "/Game/RacingGame/UI/WP_LoseScreen.WP_LoseScreen_C"))
      (`UserWidget.AddToViewport` _returnvalue_5 0)
      (set `PlayerController.bShowMouseCursor` true _returnvalue_2)
      (`WidgetBlueprintLibrary.SetInputMode_GameAndUIEx` _returnvalue_2 (`/Game/RacingGame/UI/WP_LoseScreen.Button_0` _returnvalue_5)))))

(event `Win_CrossTheFinishLine`
  (set `self.GameWon` true)
  (`self.Game Finish` true))

(event `CrossedCheckpoint`
  (params (TimeToAdd :type Integer))
  (`self.AddTimeToTimer` TimeToAdd))

(fn `AddLap`
  (params (checkpoint :type "/Game/RacingGame/Checkpoints/BP_Checkpoint Object Reference"))
  (bind _output_get (set `self.Lap` (+ (`self.Lap`) 1)))
  (`KismetSystemLibrary.PrintString` (`KismetStringLibrary.Conv_IntToString` _output_get)))

(fn `AddTimeToTimer`
  (params (TimeToAdd :type Integer))
  (bind _returnvalue (`KismetSystemLibrary.K2_SetTimerDelegate` (`|CreateDelegate` :!event `LoseOutOfTime`) (+ (`local.TimeToAdd`) (`KismetSystemLibrary.K2_GetTimerRemainingTimeHandle` (`self.TimeRemainingTimer`)))))
  (set `self.TimeRemainingTimer` _returnvalue)
  (bind _asvehicle_player_controller (cast `/Game/VehicleTemplate/Blueprints/VehiclePlayerController` (`GameplayStatics.GetPlayerController` 0)))
  (`/Game/VehicleTemplate/Blueprints/VehicleUI.PlayAddedTimeAni` (`/Game/VehicleTemplate/Blueprints/VehiclePlayerController.VehicleHud` _asvehicle_player_controller)))

(fn `UserConstructionScript`)